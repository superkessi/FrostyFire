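; Snowball actor that hits players, reacts to the environment and nudges small physics props.
; The server handles overlaps, notifying hitable actors not sharing its instigator controller and messaging physics assets through interfaces.
; Multicast events play impact effects and destroy the snowball on player or environment hits.
; Environment hits also leave a short-lived decal, with server-rolled variant, rotation and size passed along so clients match.
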(event OnComponentHit(CollisionComponent)
  (params (HitComponent :type Primitive%20Component%20Object%20Reference) (OtherActor :type Actor%20Object%20Reference) (OtherComp :type Primitive%20Component%20Object%20Reference) (NormalImpulse :type Vector :default "0, 0, 0") (Hit :type Hit%20Result%20Structure%20%28by%20ref%29))
  ;[0.1302 0.02231 0] Handle Hits (Enviroment)
  (Networking|SwitchHasAuthority
    (:Authority
      (CallFunction|MCPlayEnvironmentHitVFX (.location Hit) (.impactnormal Hit) (Class|KismetMathLibrary|RandomInteger64inRange 0 3) (Math|Random|RandomFloatinRange 0.0 3.6e+02) (Math|Random|RandomIntegerinRange 40 60)))))

(event Custom|MC_PlayHitVFX
  (params (HitLocation :type Vector))
  ;[0.009199 0.07242 0.4678] Multicast
  (Niagara|SpawnSystematLocation "/Game/VFX/FSX_SnowballExplosion.FSX_SnowballExplosion" HitLocation)
  (Actor|DestroyActor))

(event Custom|MC_PlayEnvironmentHitVFX
  (params (HitLocation :type Vector) (HitNormalhope :type Vector) (randomindexsmile :type Integer64) (randomrot :type Float%20%28double-precision%29) (randomsize :type Integer))
  ;[0.009199 0.07242 0.4678] Multicast
  (Niagara|SpawnSystematLocation "/Game/VFX/FSX_SnowballExplosionEnvironment.FSX_SnowballExplosionEnvironment" HitLocation)
  (Actor|DestroyActor)
  ;;[0.9466 0.5677 1 0.5] decal spawn 🐻✨️♡(,,>﹏<,,)♡
  (CallFunction|SpawnDecal HitLocation HitNormalhope randomindexsmile randomrot randomsize))

(event Collision|EventActorBeginOverlap
  (params (OtherActor :type Actor%20Object%20Reference))
  (bind _returnvalue (Game|GetInstigatorController))
  ;[0.4844 0.3843 0] Handle Overlaps (Players)
  (Networking|SwitchHasAuthority
    (:Authority
      (Utilities|FlowControl|Sequence
        (:then_0
          (if (and (Utilities|DoesObjectImplementInterface OtherActor "/Game/Gameplay/Interfaces/BPI_Hitable.BPI_Hitable_C") (!= (Game|GetInstigatorController OtherActor) _returnvalue))
            (bind _asbp_player_controller (Utilities|Casting|CastToBP_PlayerController _returnvalue))
            (Class|BPIHitable|OnSnowballHit(Message) OtherActor _asbp_player_controller)
            (CallFunction|MCPlayHitVFX (Transformation|GetWorldLocation (Variables|Default|GetCollisionComponent)))))
        (:then_1
          ;[0.5998 0.2658 0.9375 0.5] handle overlaps (smol assets)
          (if (Utilities|DoesObjectImplementInterface OtherActor "/Game/Assets/assetinterfaces/BPI_assetphysics.BPI_assetphysics_C")
            (Class|BPIAssetphysics|Assetphysics(Message) OtherActor)))))))

(fn ConstructionScript)

(fn SpawnDecal
  (params (Location :type Vector) (Hit%20Normal :type Vector) (Random%20Index :type Integer64) (Random%20Rotation :type Float%20%28single-precision%29) (Random%20Size :type Integer))
  (bind _returnvalue (Rendering|Material|CreateDynamicMaterialInstance "/Game/Assets/Materials/M_snowballdecal.M_snowballdecal" "None" "None" :!class /Script/Engine.KismetMaterialLibrary))
  (Rendering|Material|SetScalarParameterValue _returnvalue "Randomindex" (Math|Conversions|ToFloat(Integer) Random%20Index) :!class /Script/Engine.MaterialInstanceDynamic)
  (Rendering|Decal|SpawnDecalatLocation _returnvalue (Math|Conversions|ToVector(Float) Random%20Size) Location (Math|Rotator|CombineRotators (Math|Conversions|RotationFromXVector Hit%20Normal) (Math|Rotator|MakeRotator 0.0 Random%20Rotation 0.0)) 1e+01))