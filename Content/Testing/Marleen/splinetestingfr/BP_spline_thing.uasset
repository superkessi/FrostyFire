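; Test Blueprint that lays a chosen mesh along a spline as a row of deformed segments in the construction script.
; It adds one spline mesh per section length, with positions and tangents sampled by distance; only end tangents are clamped to that length.
; MustBeFullLengthMeshes drops the extra final segment.
; With AllowScaling on, nothing is built, and the scale-based section length logic is unconnected.
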(event EventBeginPlay)

(event Collision|EventActorBeginOverlap
  (params (OtherActor :type Actor%20Object%20Reference)))

(event EventTick
  (params (DeltaSeconds :type Float%20%28single-precision%29)))

(fn ConstructionScript
  (if (not (Variables|Default|Getallow%20scaling?))
    (if (Variables|Default|Getmust%20be%20full%20length%20meshes?)
      (for _index (range 0 (- (Math|Float|Truncate (/ (Spline|GetSplineLength (Variables|Default|GetSpline)) (Variables|Default|Getsectionlength))) 1))
        (LocalVariables|Setloop%20index _index)
        (bind _returnvalue (AddComponent|AddSplineMeshComponent false))
        (Components|StaticMesh|SetStaticMesh _returnvalue (Variables|Default|Getspline%20mesh))
        (SplineMesh|SetForwardAxis _returnvalue "X" true)
        (bind (_position _tangent) (CallFunction|GetStartPos/tan (LocalVariables|Getloop%20index)))
        (bind (_position_2 _tangent_2) (CallFunction|GetEndPos/tan (LocalVariables|Getloop%20index)))
        (SplineMesh|SetStartandEnd _returnvalue _position _tangent _position_2 _tangent_2 true :!class /Script/Engine.SplineMeshComponent))
      (else
        (for _index_2 (range 0 (Math|Float|Truncate (/ (Spline|GetSplineLength (Variables|Default|GetSpline)) (Variables|Default|Getsectionlength))))
          (LocalVariables|Setloop%20index _index_2)
          (bind _returnvalue_2 (AddComponent|AddSplineMeshComponent false))
          (Components|StaticMesh|SetStaticMesh _returnvalue_2 (Variables|Default|Getspline%20mesh))
          (SplineMesh|SetForwardAxis _returnvalue_2 "X" true)
          (bind (_position_3 _tangent_3) (CallFunction|GetStartPos/tan (LocalVariables|Getloop%20index)))
          (bind (_position_4 _tangent_4) (CallFunction|GetEndPos/tan (LocalVariables|Getloop%20index)))
          (SplineMesh|SetStartandEnd _returnvalue_2 _position_3 _tangent_3 _position_4 _tangent_4 true :!class /Script/Engine.SplineMeshComponent))))))

(fn GetStartPos/tan
  (params (index :type Integer))
  (bind _sectionlength (Variables|Default|Getsectionlength))
  (bind _returnvalue (* index _sectionlength))
  (return (Spline|GetLocationatDistanceAlongSpline (Variables|Default|GetSpline) _returnvalue "Local") (Spline|GetTangentatDistanceAlongSpline (Variables|Default|GetSpline) _returnvalue "Local")))

(fn GetEndPos/tan
  (params (index :type Integer))
  (bind _returnvalue (+ index 1))
  (bind _sectionlength (Variables|Default|Getsectionlength))
  (bind _returnvalue_2 (* _returnvalue _sectionlength))
  (return (Spline|GetLocationatDistanceAlongSpline (Variables|Default|GetSpline) _returnvalue_2 "Local") (Math|Vector|ClampVectorSize (Spline|GetTangentatDistanceAlongSpline (Variables|Default|GetSpline) _returnvalue_2 "Local") 0.0 (Variables|Default|Getsectionlength))))