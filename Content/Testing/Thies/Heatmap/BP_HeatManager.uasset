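; BP_HeatManager is a heatmap test actor that fills a Locations array with random sample points inside its area.
; The RandomLocations event repeatedly adds random points from a box centered on the actor and sized by HeatmapSize in X and Y.
; The construction script briefly draws a flat red debug box outlining that area.
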(event Custom|RandomLocations
  (bind _heatmapsize (Variables|Default|GetHeatmapSize))
  (bind _returnvalue (/ _heatmapsize 2.0))
  (for _index (range 0 100)
    (Utilities|Array|Add (Variables|Default|GetLocations) (Math|Random|RandomPointinBoundingBox (Transformation|GetActorLocation) (Math|Vector|MakeVector _returnvalue _returnvalue 0.0)))))

(event EventBeginPlay)

(fn ConstructionScript
  (bind _heatmapsize (Variables|Default|GetHeatmapSize))
  (bind _returnvalue (/ _heatmapsize 2.0))
  (Rendering|Debug|DrawDebugBox (Transformation|GetActorLocation) (Math|Vector|MakeVector _returnvalue _returnvalue 1.0) "(R=1.000000,G=0.010032,B=0.000000,A=1.000000)" "0, 0, 0" 1.0 1.0))