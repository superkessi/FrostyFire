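; BP_HeatNodes is a heat point actor for a heatmap test, shown as a sphere with a dynamic M_HeatPoint material.
; The construction script scales the actor by OverlapRadius / 50 and stores the material instance in PointMaterial.
; CalculateHeat runs a sphere overlap for other heat nodes within that radius, but is unfinished: the result and its MaxOverlaps input go unused.
; The event graph is empty.
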(event EventBeginPlay)

(event Collision|EventActorBeginOverlap
  (params (OtherActor :type Actor%20Object%20Reference)))

(event EventTick
  (params (DeltaSeconds :type Float%20%28single-precision%29)))

(fn ConstructionScript
  (Transformation|SetActorScale3D (Math|Conversions|ToVector(Float) (/ (Variables|Default|GetOverlapRadius) 5e+01)))
  (bind _returnvalue (Rendering|Material|CreateDynamicMaterialInstance (Variables|Default|GetSphere) 0 "/Game/Testing/Thies/Heatmap/M_HeatPoint.M_HeatPoint" "None" :!class /Script/Engine.PrimitiveComponent))
  (Variables|Default|SetPointMaterial _returnvalue))

(fn CalculateHeat
  (params (MaxOverlaps :type Integer))
  (Collision|SphereOverlapActors (Transformation|GetActorLocation) (Variables|Default|GetOverlapRadius) (Utilities|Array|MakeArray "ObjectTypeQuery2") "BP_HeatNodes_C"))