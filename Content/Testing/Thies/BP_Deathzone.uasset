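; Test deathzone actor with a box trigger that kills and respawns players who overlap it, with a water splash effect at their location.
; On overlap it resolves the actor's BP_PlayerState through its instigator controller and passes it to GM_Base's KillPlayer and RequestRespawn.
; An older GM_LastManStanding branch that subtracts lives and reports player death is left disconnected and never runs.
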(event OnComponentBeginOverlap(Box)
  (params (OverlappedComponent :type Primitive%20Component%20Object%20Reference) (OtherActor :type Actor%20Object%20Reference) (OtherComp :type Primitive%20Component%20Object%20Reference) (OtherBodyIndex :type Integer) (bFromSweep :type Boolean) (SweepResult :type Hit%20Result%20Structure%20%28by%20ref%29))
  (bind _asbp_player_state (CallFunction|GetActorPlayerState OtherActor))
  ;[0.1302 0.1302 0.1302] Deathzone (Should cast an command when overlaping the collision box of bp)
  (Default|KillPlayer (CallFunction|GetGameModeBase) 0 _asbp_player_state)
  (Default|RequestRespawn (CallFunction|GetGameModeBase) _asbp_player_state)
  (CallFunction|PlayWaterFX (Transformation|GetActorLocation OtherActor)))

(event Custom|PlayWaterFX
  (params (Location :type Vector))
  ;[0.1302 0.1302 0.1302] Deathzone (Should cast an command when overlaping the collision box of bp)
  (Niagara|SpawnSystematLocation "/Game/VFX/FSX_WaterSpash.FSX_WaterSpash" Location))

(fn ConstructionScript)

(fn GetActorPlayerState
  (params (Target :type Actor%20Object%20Reference))
  (bind _asbp_player_controller (Utilities|Casting|CastToBP_PlayerController (Game|GetInstigatorController Target))
    (:then
      (bind _asbp_player_state (Utilities|Casting|CastToBP_PlayerState (Variables|/Script/Engine.Controller|GetPlayerState _asbp_player_controller))))
    (:CastFailed
      _))
  (return _asbp_player_state))

(fn GetGameModeBase
  (bind _asgm_base (Utilities|Casting|CastToGM_Base (Game|GetGameMode)))
  (Utilities|IsValid _asgm_base
    (:Is%20Valid
      (return _asgm_base))))