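; Test snowball projectile that notifies hittable actors it strikes and bursts on impact.
; On the server, overlaps with BPI_Hitable actors other than the thrower send a hit message carrying the thrower's BP_PlayerController, while collision component hits cover the environment.
; Both paths call a multicast event that spawns the snowball explosion effect at the impact and destroys the actor.
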(event OnComponentHit(CollisionComponent)
  (params (HitComponent :type Primitive%20Component%20Object%20Reference) (OtherActor :type Actor%20Object%20Reference) (OtherComp :type Primitive%20Component%20Object%20Reference) (NormalImpulse :type Vector :default "0, 0, 0") (Hit :type Hit%20Result%20Structure%20%28by%20ref%29))
  ;[0.1302 0.02231 0] Handle Hits (Enviroment)
  (Networking|SwitchHasAuthority
    (:Authority
      (CallFunction|MCPlayHitVFX (.location Hit)))))

(event Custom|MC_PlayHitVFX
  (params (HitLocation :type Vector))
  ;[0.009199 0.07242 0.4678] Multicast
  (Niagara|SpawnSystematLocation "/Game/VFX/FSX_SnowballExplosion.FSX_SnowballExplosion" HitLocation)
  (Actor|DestroyActor))

(event EventBeginPlay)

(event Collision|EventActorBeginOverlap
  (params (OtherActor :type Actor%20Object%20Reference))
  (bind _returnvalue (Game|GetInstigatorController))
  ;[0.4844 0.3843 0] Handle Overlaps (Players)
  (Networking|SwitchHasAuthority
    (:Authority
      (if (Utilities|DoesObjectImplementInterface OtherActor "/Game/Gameplay/Interfaces/BPI_Hitable.BPI_Hitable_C")
        (if (not (== (Game|GetInstigatorController OtherActor) _returnvalue))
          (bind _asbp_player_controller (Utilities|Casting|CastToBP_PlayerController _returnvalue))
          (Class|BPIHitable|OnSnowballHit(Message) OtherActor _asbp_player_controller)
          (CallFunction|MCPlayHitVFX (Transformation|GetWorldLocation (Variables|Default|GetCollisionComponent))))))))

(fn ConstructionScript)