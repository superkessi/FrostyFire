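; BP_cocktail is a cocktail prop that can be knocked loose with physics and respawns at its original spot.
; BeginPlay stores the starting transform, and Assetphysics relays through a server event to a multicast event.
; The multicast enables mesh physics, plays a glass-and-wood hit sound at the start location, then disables physics and restores the transform after a ten-second delay.
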(event Custom|server%20assetphysics
  ;[1 0.8148 0.4793] brieftauben
  (CallFunction|McAssetphysics))

(event Custom|mc%20assetphysics
  ;[0.9911 0.6867 0.7835] wundervoller multicast der physics an macht und             dann sound und dann                                                                                                                                                    respawned nach 10s
  (Physics|SetSimulatePhysics (Variables|Default|Getmeshmeowmeow) true)
  (Audio|PlaySoundatLocation "/Game/Audio/Snowball/Cue/SFX_hitglassandwood_Cue.SFX_hitglassandwood_Cue" (Variables|Default|GetStart%20Location) (Variables|Default|GetStart%20Rotation) 1.0 1.0 0.0 0 0 0 0)
  (Utilities|FlowControl|Delay 1e+01)
  (Physics|SetSimulatePhysics (Variables|Default|Getmeshmeowmeow) false)
  (Transformation|SetActorLocationAndRotation (Variables|Default|GetStart%20Location) (Variables|Default|GetStart%20Rotation)))

(event EventBeginPlay
  ;[0.5972 0.7605 0.8228] speichert wundervoll startlocation und rotation
  (Variables|Default|SetStart%20Location (Transformation|GetActorLocation))
  (Variables|Default|SetStart%20Rotation (Transformation|GetActorRotation)))

(event Collision|EventActorBeginOverlap
  (params (OtherActor :type Actor%20Object%20Reference)))

(event EventTick
  (params (DeltaSeconds :type Float%20%28single-precision%29)))

(event EventAssetphysics
  ;[1 0.8148 0.4793] brieftauben
  (CallFunction|ServerAssetphysics))

(fn ConstructionScript)