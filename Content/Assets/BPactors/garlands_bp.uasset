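; Garland actor that builds a chain of spline meshes along its spline and animates the spline points over time.
; The construction script adds a spline mesh per point, shaped by local positions and tangents to the next point.
; Tick scales each point's current world location by a speed-driven sine, from a variable start index, compounding each frame.
; Tick never updates the spline meshes themselves.
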(event EventBeginPlay)

(event Collision|EventActorBeginOverlap
  (params (OtherActor :type Actor%20Object%20Reference)))

(event EventTick
  (params (DeltaSeconds :type Float%20%28single-precision%29))
  (for _index (range (Math|Float|Truncate (Variables|Default|Getchattivarwtf)) (Spline|GetNumberOfSplinePoints (Variables|Default|GetSpline)))
    (Spline|SetLocationatSplinePoint (Variables|Default|GetSpline) _index (* (Spline|GetLocationatSplinePoint (Variables|Default|GetSpline) _index "World") (* (Math|Trig|Sin(Radians) (* (Utilities|Time|GetGameTimeinSeconds) (Variables|Default|Getspeed))) "1.000000,1.000000,1.000000")) "World" true)))

(fn ConstructionScript
  (for _index (range 0 (- (Spline|GetNumberOfSplinePoints (Variables|Default|GetSpline)) 1))
    (bind _returnvalue (AddComponent|AddSplineMeshComponent false))
    (SplineMesh|SetStartandEnd _returnvalue (Spline|GetLocationatSplinePoint (Variables|Default|GetSpline) _index "Local") (Spline|GetTangentatSplinePoint (Variables|Default|GetSpline) _index "Local") (Spline|GetLocationatSplinePoint (Variables|Default|GetSpline) (+ _index 1) "Local") (Spline|GetTangentatSplinePoint (Variables|Default|GetSpline) (+ _index 1) "Local") true :!class /Script/Engine.SplineMeshComponent)))