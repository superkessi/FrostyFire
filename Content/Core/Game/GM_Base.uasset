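; Base multiplayer game mode that runs shared match flow and leaves hit handling, game-over and winner rules as stubs for child modes.
; Once all players are ready, it advances the match phase on GS_Base and runs a one-second looping countdown timer.
; Kills multicast death feedback and killfeed through the victim's character and game state.
; Respawn requests start a timer on the player controller, and respawns use random PlayerStarts.
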(event Custom|HandlePlayerHit
  (params (AttackerController :type BP%20Player%20Controller%20Object%20Reference) (VictimController :type BP%20Player%20Controller%20Object%20Reference))
  ;[0.001741 0.01371 0.08854] Events to Implement in Children
  (Development|PrintString "GM : Hit not implementet"))

(event Custom|StartCountDown
  (bind _gamestate (Getter|GetGameStateBase))
  ;[0.4844 0.3843 0] Starting Countdown
  (Default|CallOnStartGame)
  (Variables|/Game/Core/Game/GS_Base.GS_Base_C|SetMatchPhase _gamestate "NewEnumerator1")
  (Variables|/Game/Core/Game/GS_Base.GS_Base_C|SetCountdownTime _gamestate (Variables|/Game/Core/Game/GS_Base.GS_Base_C|GetMaxCountdownTime _gamestate))
  (bind _returnvalue (Utilities|Time|SetTimerbyEvent (delegate Custom|CountdownTick) 1.0 true)))

(event Custom|CountdownTick
  (bind _gamestate (Getter|GetGameStateBase))
  ;[0.4844 0.3843 0] Starting Countdown
  (if (>= (- (Variables|/Game/Core/Game/GS_Base.GS_Base_C|GetCountdownTime _gamestate) 1) 0)
    (Variables|/Game/Core/Game/GS_Base.GS_Base_C|SetCountdownTime _gamestate (- (Variables|/Game/Core/Game/GS_Base.GS_Base_C|GetCountdownTime _gamestate) 1))
    (else
      (Utilities|Time|ClearandInvalidateTimerbyHandle (stale Custom|StartCountDown _returnvalue)))))

(event Custom|OnStartTimerEnd
  ;[0.001741 0.01371 0.08854] Events to Implement in Children
  (Development|PrintString "GM : Start Timer End not implementet"))

(event Custom|KillPlayer
  (params (KillerState :type BP%20Player%20State%20Object%20Reference) (TargetState :type BP%20Player%20State%20Object%20Reference))
  (bind _asbp_player_character (Utilities|Casting|CastToBP_PlayerCharacter (PlayerState|GetPawn TargetState)))
  (Default|MCPlayDeathFeedback _asbp_player_character)
  (CallFunction|ShowKillfeed KillerState TargetState))

(event Custom|ShowKillfeed
  (params (Attacker :type BP%20Player%20State%20Object%20Reference) (Victim :type BP%20Player%20State%20Object%20Reference))
  (Default|MCShowKillfeed (Getter|GetGameStateBase) Attacker Victim))

(event Custom|RespawnPlayer
  (params (TargetState :type BP%20Player%20State%20Object%20Reference))
  (bind _asbp_player_controller (Utilities|Casting|CastToBP_PlayerController (Components|GetOwner TargetState)))
  (Pawn|UnPossess _asbp_player_controller)
  (Class|GameModeBase|RestartPlayeratPlayerStart _asbp_player_controller (Game|GetRandomSpawn))
  (Default|ActivatePlayer (Default|GetCharacter _asbp_player_controller) true))

(event Custom|StartRound
  ;[0.1302 0.02231 0] Start Setup
  (Class|GameMode|StartMatch)
  (Variables|/Game/Core/Game/GS_Base.GS_Base_C|SetMatchPhase (Getter|GetGameStateBase) "NewEnumerator0"))

(event Custom|RequestRespawn
  (params (TargetState :type BP%20Player%20State%20Object%20Reference))
  (bind _asbp_player_controller (Utilities|Casting|CastToBP_PlayerController (Components|GetOwner TargetState)))
  (Default|ServerStartRespawnTimer _asbp_player_controller))

(event EventBeginPlay
  ;[0.1302 0.02231 0] Start Setup
  (CallFunction|StartRound))

(fn ConstructionScript)

(fn ChoosePlayerStart
  (params (Player :type Controller%20Object%20Reference))
  (bind _outactors (Actor|GetAllActorsOfClass "/Script/Engine.PlayerStart"))
  (Development|PrintText (Utilities|Text|FormatText "SpawnID : {ID}" (.OutIndex (Utilities|Array|Random _outactors))) false false)
  (return (.OutItem (Utilities|Array|Random _outactors))))

(fn SetStates
  (params (AttackerController :type Controller%20Object%20Reference) (VictimController :type Controller%20Object%20Reference))
  (Utilities|FlowControl|Sequence
    (:then_0
      (Variables|HitDetection|SetAttackerState 0)
      (bind _asbp_player_state (Utilities|Casting|CastToBP_PlayerState (Variables|/Script/Engine.Controller|GetPlayerState AttackerController)))
      (Variables|HitDetection|SetAttackerState _asbp_player_state))
    (:then_1
      (Variables|HitDetection|SetVictimState 0)
      (bind _asbp_player_state_2 (Utilities|Casting|CastToBP_PlayerState (Variables|/Script/Engine.Controller|GetPlayerState VictimController)))
      (Variables|HitDetection|SetVictimState _asbp_player_state_2))))

(fn CheckifGameOver
  (Development|PrintString "GM: CheckGameOver not implemented")
  (return false))

(fn RestartMatch
  (Class|GameMode|RestartGame))

(fn GetGameStateBase
  (bind _asgs_base (Utilities|Casting|CastToGS_Base (Game|GetGameState)))
  (return _asgs_base))

(fn GetRandomSpawn
  (bind _outactors (Actor|GetAllActorsOfClass "/Script/Engine.PlayerStart"))
  (return (.OutItem (Utilities|Array|Random _outactors))))

(fn DetermineWinner
  (Development|PrintText "DetermineWinner NOT IMPLEMENTED in GameMode!!!"))

(fn DetermineWinningOrder
  (Development|PrintText "SetWinningOrder NOT IMPLEMENTED in GameMode!!!"))

(fn CheckAllPlayersReady
  (if (== (Variables|/Game/Core/Game/GS_Base.GS_Base_C|GetMatchPhase (Getter|GetGameStateBase)) (Math|Conversions|ToInteger(Byte) (Utilities|Enum|LiteralenumENUM_MatchPhases "NewEnumerator0")))
    (for _array_element (Variables|/Script/Engine.GameStateBase|GetPlayerArray (Game|GetGameState))
      (bind _asbp_player_state (Utilities|Casting|CastToBP_PlayerState _array_element))
      (if (not (Variables|/Game/Core/Player/BP_PlayerState.BP_PlayerState_C|GetIsReady _asbp_player_state))
        (return)))
    (CallFunction|StartCountDown)))