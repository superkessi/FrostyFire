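; Game mode for a timed deathmatch without lives, where each player hit scores a kill, kills the victim and requests their respawn.
; After the start timer ends, a one-second looping timer counts down the match time stored in the game state.
; At expiry, a selection sort on kill score sets the winning order and winner, then changes match phase.
; Pawn classes come from game-instance character selections keyed by player name, defaulting to BP_PlayerCharacter.
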(event Custom|StartMatchTimer
  (bind _gamestate (Getter|GetTDMState))
  ;[0.009199 0.07242 0.4678] Match Timer
  (Variables|/Game/Core/Game/GS_Base.GS_Base_C|SetMatchPhase (CallFunction|GetGameStateBase) "NewEnumerator2")
  (Variables|/Game/Core/Game/GS_TimedDeathmatch.GS_TimedDeathmatch_C|SetRemainingMatchTime _gamestate (Variables|/Game/Core/Game/GS_TimedDeathmatch.GS_TimedDeathmatch_C|GetMaxMatchTime _gamestate))
  (bind _returnvalue (Utilities|Time|SetTimerbyEvent (delegate Custom|MatchTimerTick) 1.0 true)))

(event Custom|MatchTimerTick
  (bind _gamestate (Getter|GetTDMState))
  ;[0.009199 0.07242 0.4678] Match Timer
  (if (>= (- (Variables|/Game/Core/Game/GS_TimedDeathmatch.GS_TimedDeathmatch_C|GetRemainingMatchTime _gamestate) 1) 0)
    (Variables|/Game/Core/Game/GS_TimedDeathmatch.GS_TimedDeathmatch_C|SetRemainingMatchTime _gamestate (Math|Conversions|ToFloat(Integer) (- (Variables|/Game/Core/Game/GS_TimedDeathmatch.GS_TimedDeathmatch_C|GetRemainingMatchTime _gamestate) 1)))
    (else
      (Utilities|Time|ClearandInvalidateTimerbyHandle (stale Custom|StartMatchTimer _returnvalue))
      (CallFunction|MConMatchTimerEnd))))

(event Custom|MC_OnMatchTimerEnd
  (CallFunction|DetermineWinningOrder)
  (CallFunction|DetermineWinner)
  (Variables|/Game/Core/Game/GS_Base.GS_Base_C|SetMatchPhase (CallFunction|GetGameStateBase) "NewEnumerator3"))

(event EventHandlePlayerHit
  (params (AttackerController :type BP%20Player%20Controller%20Object%20Reference) (VictimController :type BP%20Player%20Controller%20Object%20Reference))
  (bind _victimstate (Variables|Default|GetVictimState))
  (CallFunction|SetStates AttackerController VictimController)
  (CallFunction|UpdatePlayerScores)
  (Default|PlayHitMarker (Getter|GetCharacter (Variables|Default|GetAttackerState)) true)
  (CallFunction|KillPlayer (Variables|Default|GetAttackerState) _victimstate)
  (CallFunction|RequestRespawn _victimstate))

(event EventOnStartTimerEnd
  (CallFunction|StartMatchTimer))

(fn ConstructionScript
  (|CallParentFunction))

(fn GetTDMState
  (return (.AsGS%20Timed%20Deathmatch (Utilities|Casting|CastToGS_TimedDeathmatch (CallFunction|GetGameStateBase)))))

(fn UpdatePlayerScores
  (Default|AddScore (Variables|Default|GetAttackerState) 1)
  (Default|AddDeath (Variables|Default|GetVictimState)))

(fn GetDefaultPawnClassforController
  (params (InController :type Controller%20Object%20Reference))
  (bind _returnvalue (Game|GetGameInstance))
  (bind _playerstate (Variables|/Script/Engine.Controller|GetPlayerState InController))
  (bind _returnvalue_2 (PlayerState|GetPlayerName _playerstate))
  (bind _asbp_afgame_instance (Utilities|Casting|CastToBP_AFGameInstance _returnvalue))
  (bind _selectedcharactersofallplayers (Variables|/Game/Core/Game/BP_AFGameInstance.BP_AFGameInstance_C|GetSelectedCharactersOfAllPlayers _asbp_afgame_instance))
  (bind _value (Utilities|Map|Find _selectedcharactersofallplayers _returnvalue_2))
  (if (Utilities|IsValidClass _value)
    (return _value)
    (else
      (return "/Game/Core/Player/BP_PlayerCharacter.BP_PlayerCharacter_C"))))

(fn DetermineWinner
  (bind _gamestate (CallFunction|GetGameStateBase))
  (Variables|/Game/Core/Game/GS_Base.GS_Base_C|SetWinner _gamestate (Utilities|Array|Get(acopy) (Variables|/Game/Core/Game/GS_Base.GS_Base_C|GetWinningOrder _gamestate))))

(fn DetermineWinningOrder
  (Utilities|Array|Clear (LocalVariables|GetUnsortedPlayers))
  (LocalVariables|SetUnsortedPlayers (Variables|/Script/Engine.GameStateBase|GetPlayerArray (CallFunction|GetGameStateBase)))
  (if (> (Utilities|Array|Length (LocalVariables|GetUnsortedPlayers)) 0) :!label _label
    (LocalVariables|SetCurrentPlayerState (.AsBP%20Player%20State (Utilities|Casting|CastToBP_PlayerState (.OutItem (Utilities|Array|Random (LocalVariables|GetUnsortedPlayers))))))
    (for _array_element (LocalVariables|GetUnsortedPlayers)
      (bind _asbp_player_state (Utilities|Casting|CastToBP_PlayerState _array_element))
      (if (> (Variables|/Game/Core/Player/BP_PlayerState.BP_PlayerState_C|GetKillScore _asbp_player_state) (Variables|/Game/Core/Player/BP_PlayerState.BP_PlayerState_C|GetKillScore (LocalVariables|GetCurrentPlayerState)))
        (LocalVariables|SetCurrentPlayerState _asbp_player_state)))
    (Utilities|Array|RemoveItem (LocalVariables|GetUnsortedPlayers) (LocalVariables|GetCurrentPlayerState))
    (Utilities|Array|AddUnique (LocalVariables|GetSortedPlayers) (LocalVariables|GetCurrentPlayerState))
    (goto _label)
    (else
      (Variables|/Game/Core/Game/GS_Base.GS_Base_C|SetWinningOrder (CallFunction|GetGameStateBase) (LocalVariables|GetSortedPlayers)))))

(fn GetCharacter
  (params (Target :type BP%20Player%20State%20Object%20Reference))
  (return (.AsBP%20Player%20Character (Utilities|Casting|CastToBP_PlayerCharacter (PlayerState|GetPawn Target)))))