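; Game mode for Last Man Standing matches, spawning each player as their selected character from the game instance, with a default fallback.
; Each hit removes a life from the victim and plays feedback; a death scores the attacker and moves the victim into a spectator pawn.
; When one or fewer players remain alive, it records the winner, sets WinningOrder to an empty array and advances the GameState's match phase.
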(event Custom|OnGameOver
  (CallFunction|DetermineWinningOrder)
  (CallFunction|DetermineWinner)
  (Variables|/Game/Core/Game/GS_Base.GS_Base_C|SetMatchPhase (CallFunction|GetGameStateBase) "NewEnumerator3"))

(event Custom|OnPlayerDied
  (bind _attackerstate (Variables|Default|GetAttackerState))
  (if (Utilities|IsValid _attackerstate)
    (Default|AddScore _attackerstate 1))
  (CallFunction|KillPlayer (Variables|Default|GetAttackerState) (Variables|Default|GetVictimState))
  (CallFunction|SwitchtoSpectatorCam)
  (bind _gameover (CallFunction|CheckifGameOver))
  (if _gameover
    (CallFunction|OnGameOver)))

(event EventOnStartTimerEnd
  (Variables|/Game/Core/Game/GS_Base.GS_Base_C|SetMatchPhase (CallFunction|GetGameStateBase) "NewEnumerator2"))

(event EventHandlePlayerHit
  (params (AttackerController :type BP%20Player%20Controller%20Object%20Reference) (VictimController :type BP%20Player%20Controller%20Object%20Reference))
  (bind _victimstate (Variables|Default|GetVictimState))
  (CallFunction|SetStates AttackerController VictimController)
  (Default|SubstactLive _victimstate 1)
  (if (Variables|/Game/Core/Player/BP_PlayerState.BP_PlayerState_C|GetIsDead _victimstate)
    (CallFunction|OnPlayerDied)
    (Default|PlayHitMarker (Getter|GetCharacter (Variables|Default|GetAttackerState)) true)
    (else
      (Default|MCPlayHitFeedback (Getter|GetCharacter (Variables|Default|GetVictimState)))
      (Default|PlayHitMarker (Getter|GetCharacter (Variables|Default|GetAttackerState)) false))))

(fn ConstructionScript
  (|CallParentFunction))

(fn CheckifGameOver
  (CallFunction|CheckRemainingPlayers)
  (if (<= (Utilities|Array|Length (Variables|Default|GetPlayersAlive)) 1)
    (Variables|/Game/Core/Game/GS_Base.GS_Base_C|SetWinner (CallFunction|GetGameStateBase) (Utilities|Array|Get(acopy) (Variables|Default|GetPlayersAlive)))
    (return true)
    (else
      (return false))))

(fn CheckRemainingPlayers
  (Utilities|Array|Clear (Variables|Default|GetPlayersAlive))
  (for _array_element (Variables|/Script/Engine.GameStateBase|GetPlayerArray (Game|GetGameState))
    (bind _asbp_player_state (Utilities|Casting|CastToBP_PlayerState _array_element))
    (if (not (Variables|/Game/Core/Player/BP_PlayerState.BP_PlayerState_C|GetIsDead _asbp_player_state))
      (Utilities|Array|AddUnique (Variables|Default|GetPlayersAlive) _asbp_player_state))))

(fn GetDefaultPawnClassforController
  (params (InController :type Controller%20Object%20Reference))
  (bind _returnvalue (Game|GetGameInstance))
  (bind _playerstate (Variables|/Script/Engine.Controller|GetPlayerState InController))
  (bind _returnvalue_2 (PlayerState|GetPlayerName _playerstate))
  (bind _asbp_afgame_instance (Utilities|Casting|CastToBP_AFGameInstance _returnvalue))
  (bind _selectedcharactersofallplayers (Variables|/Game/Core/Game/BP_AFGameInstance.BP_AFGameInstance_C|GetSelectedCharactersOfAllPlayers _asbp_afgame_instance))
  (bind _value (Utilities|Map|Find _selectedcharactersofallplayers _returnvalue_2))
  (if (Utilities|IsValidClass _value)
    (return _value)
    (else
      (return "/Game/Core/Player/BP_PlayerCharacter.BP_PlayerCharacter_C"))))

(fn SwitchtoSpectatorCam
  (bind _victimstate (Variables|Default|GetVictimState))
  (bind _returnvalue (Game|GetPlayerController _victimstate))
  (bind _output_get (LocalVariables|SetRespawnPos (Math|Conversions|ToTransform(Vector) (Transformation|GetActorLocation (PlayerState|GetPawn _victimstate)))))
  (Pawn|UnPossess _returnvalue)
  (bind _returnvalue_2 (Game|SpawnActorfromClass "/Game/Core/Player/BP_SpectatorCharacter.BP_SpectatorCharacter_C" _output_get "Undefined" "MultiplyWithRoot" 0 0))
  (Pawn|Possess _returnvalue _returnvalue_2))

(fn DetermineWinner
  (CallFunction|CheckRemainingPlayers)
  (Variables|/Game/Core/Game/GS_Base.GS_Base_C|SetWinner (CallFunction|GetGameStateBase) (Utilities|Array|Get(acopy) (Variables|Default|GetPlayersAlive))))

(fn DetermineWinningOrder
  (Variables|/Game/Core/Game/GS_Base.GS_Base_C|SetWinningOrder (CallFunction|GetGameStateBase) (LocalVariables|GetEmptyArray)))

(fn GetCharacter
  (params (TargetState :type BP%20Player%20State%20Object%20Reference))
  (return (.AsBP%20Player%20Character (Utilities|Casting|CastToBP_PlayerCharacter (PlayerState|GetPawn TargetState)))))