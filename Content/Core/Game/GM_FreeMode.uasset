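; Free-mode game mode that runs a timed match with life-based scoring, using the GS_TimedDeathmatch game state.
; When the start timer ends, it sets the match phase and counts remaining time down each second; a match-end event advances the phase.
; Hits cost victims a life, and losing all awards the attacker a point, then kills and respawns the victim.
; Pawn classes come from game-instance selections keyed by player name, defaulting to BP_PlayerCharacter.
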(event Custom|StartMatchTimer
  (bind _gamestate (Getter|GetTDMState))
  ;[0.009199 0.07242 0.4678] Match Timer
  (Variables|/Game/Core/Game/GS_Base.GS_Base_C|SetMatchPhase (CallFunction|GetGameStateBase) "NewEnumerator2")
  (Variables|/Game/Core/Game/GS_TimedDeathmatch.GS_TimedDeathmatch_C|SetRemainingMatchTime _gamestate (Variables|/Game/Core/Game/GS_TimedDeathmatch.GS_TimedDeathmatch_C|GetMaxMatchTime _gamestate))
  (Utilities|Time|SetTimerbyEvent (delegate Custom|MatchTimerTick) 1.0 true))

(event Custom|MatchTimerTick
  (bind _gamestate (Getter|GetTDMState))
  ;[0.009199 0.07242 0.4678] Match Timer
  (if (>= (- (Variables|/Game/Core/Game/GS_TimedDeathmatch.GS_TimedDeathmatch_C|GetRemainingMatchTime _gamestate) 1) 0)
    (Variables|/Game/Core/Game/GS_TimedDeathmatch.GS_TimedDeathmatch_C|SetRemainingMatchTime _gamestate (Math|Conversions|ToFloat(Integer) (- (Variables|/Game/Core/Game/GS_TimedDeathmatch.GS_TimedDeathmatch_C|GetRemainingMatchTime _gamestate) 1)))))

(event Custom|OnMatchTimerEnd
  (Variables|/Game/Core/Game/GS_Base.GS_Base_C|SetMatchPhase (CallFunction|GetGameStateBase) "NewEnumerator3"))

(event EventOnStartTimerEnd
  (CallFunction|StartMatchTimer))

(fn ConstructionScript
  (|CallParentFunction))

(fn GetTDMState
  (return (.AsGS%20Timed%20Deathmatch (Utilities|Casting|CastToGS_TimedDeathmatch (CallFunction|GetGameStateBase)))))

(fn UpdatePlayerScores
  (bind _victimstate (Variables|Default|GetVictimState))
  (Default|SubstactLive _victimstate 1)
  (if (Variables|/Game/Core/Player/BP_PlayerState.BP_PlayerState_C|GetIsDead _victimstate)
    (Default|AddScore (Variables|Default|GetAttackerState) 1)
    (CallFunction|KillVictim)
    (CallFunction|RespawnVictim)))

(fn KillVictim
  (bind _victimstate (Variables|Default|GetVictimState))
  (bind _returnvalue (PlayerState|GetPawn _victimstate))
  (Utilities|IsValid _returnvalue
    (:Is%20Valid
      (bind _asbp_player_character (Utilities|Casting|CastToBP_PlayerCharacter _returnvalue))
      (Default|Die _asbp_player_character))))

(fn RespawnVictim
  (bind _victimstate (Variables|Default|GetVictimState))
  (Default|ResetPlayerLives _victimstate)
  (bind _asbp_player_controller (Utilities|Casting|CastToBP_PlayerController (Components|GetOwner _victimstate)))
  (Pawn|UnPossess _asbp_player_controller)
  (Class|GameModeBase|RestartPlayer _asbp_player_controller)
  (Default|ActivatePlayer (Default|GetCharacter _asbp_player_controller) true))

(fn GetDefaultPawnClassforController
  (params (InController :type Controller%20Object%20Reference))
  (bind _returnvalue (Game|GetGameInstance))
  (bind _playerstate (Variables|/Script/Engine.Controller|GetPlayerState InController))
  (bind _returnvalue_2 (PlayerState|GetPlayerName _playerstate))
  (bind _asbp_afgame_instance (Utilities|Casting|CastToBP_AFGameInstance _returnvalue))
  (bind _selectedcharactersofallplayers (Variables|/Game/Core/Game/BP_AFGameInstance.BP_AFGameInstance_C|GetSelectedCharactersOfAllPlayers _asbp_afgame_instance))
  (bind _value (Utilities|Map|Find _selectedcharactersofallplayers _returnvalue_2))
  (if (Utilities|IsValidClass _value)
    (return _value)
    (else
      (return "/Game/Core/Player/BP_PlayerCharacter.BP_PlayerCharacter_C"))))