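; Game instance that owns the player's persistent settings and manages multiplayer session hosting, joining and leaving.
; On init it loads or creates the settings save and applies volumes through a sound mix; setters for mouse sensitivity and volume update and save it.
; Advanced Sessions creates 8-player sessions that open the lobby or fun level as listen servers.
; Invites trigger joins; network and travel errors destroy the session.
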(event Custom|Create%20Session
  ;[0.08415 0.4678 0.04761] Session Logic
  (|CreateSession))

(event Custom|LeaveSession
  ;[0.08415 0.4678 0.04761] Session Logic
  (Game|OpenLevel(byObjectReference) "/Game/Levels/LVL_MainMenu.LVL_MainMenu")
  (|DestroySession (Game|GetPlayerController 0)))

(event Custom|CreateLobbySession
  ;[0.08415 0.4678 0.04761] Session Logic
  (|CreateLobby))

(event EventHandleNetworkError
  (params (FailureType :type ENetworkFailure%20Enum :default "NetDriverAlreadyExists") (bIsServer :type Boolean))
  ;[0.8281 0 0.07523] Debugging
  (Development|PrintString (Utilities|String|EnumtoString FailureType))
  (|DestroySession (Game|GetPlayerController 0)))

(event EventHandleTravelError
  (params (FailureType :type ETravelFailure%20Enum :default "NoLevel"))
  ;[0.8281 0 0.07523] Debugging
  (Development|PrintString (Utilities|String|EnumtoString FailureType))
  (|DestroySession (Game|GetPlayerController 0)))

(event EventOnSessionInviteAccepted
  (params (LocalPlayerNum :type Integer) (PersonInvited :type BP%20Unique%20Net%20Id%20Structure) (SessionToJoin :type Blueprint%20Session%20Result%20Structure%20%28by%20ref%29))
  ;[0.1597 0.05208 0.4678] Client join Session
  (|JoinSession (Game|GetPlayerController 0) SessionToJoin))

(event EventInit
  ;[0.1879 0.3277 0.4678] Save System
  (Settings|LoadSettings)
  (ApplySettings|SetInitialVolumes))

(event EventShutdown
  ;[0.1879 0.3277 0.4678] Save System
  (Settings|SaveSettings))

(fn LoadSettings
  (bind _returnvalue (SaveGame|LoadGamefromSlot (Variables|Settings|GetSettingSlot)))
  (bind _assav_settings (Utilities|Casting|CastToSAV_Settings _returnvalue)
    (:then
      (Variables|Settings|SetSettings _assav_settings))
    (:CastFailed
      ;[0.8281 0 0.07523] Create if not found
      (bind _returnvalue_2 (SaveGame|CreateSaveGameObject "/Game/Core/Data/SAV_Settings.SAV_Settings_C"))
      (bind _returnvalue_3 (SaveGame|SaveGametoSlot _returnvalue_2 (Variables|Settings|GetSettingSlot)))
      (if _returnvalue_3
        (Settings|LoadSettings)
        (else
          (Development|PrintString "ERROR: Failed to create Settings Save"))))))

(fn SaveSettings
  (bind _returnvalue (SaveGame|SaveGametoSlot (Variables|Settings|GetSettings) (Variables|Settings|GetSettingSlot)))
  ;[0.8281 0 0.07523] Debugging
  (if (not _returnvalue)
    (Development|PrintString "ERROR: Failed to safe settings!")))

(fn UpdateMouseSens
  (params (NewSens :type Float%20%28double-precision%29))
  (bind _output_get (Variables|/Game/Core/Data/SAV_Settings.SAV_Settings_C|SetMouseSensitivity (Variables|Settings|GetSettings) NewSens))
  (bind _asbp_player_character (Utilities|Casting|CastToBP_PlayerCharacter (Pawn|GetControlledPawn (Game|GetPlayerController 0)))
    (:then
      (Variables|/Script/FrostyFire.FrostyFireCharacter|SetMouseSensitivity _asbp_player_character _output_get)
      (Settings|SaveSettings))
    (:CastFailed
      (Development|PrintString "PC cast failed"))))

(fn UpdateMusicVolume
  (params (NewVolume :type Float%20%28double-precision%29))
  (bind _output_get (Variables|/Game/Core/Data/SAV_Settings.SAV_Settings_C|SetMusicVolume (Variables|Settings|GetSettings) NewVolume))
  (Audio|SetSoundMixClassOverride "/Game/Audio/MIX_Main.MIX_Main" "/Game/Audio/SC_Music.SC_Music" _output_get 1.0 0.1 true)
  (Audio|PushSoundMixModifier "/Game/Audio/MIX_Main.MIX_Main")
  (Settings|SaveSettings))

(fn UpdateSoundVolume
  (params (NewVolume :type Float%20%28double-precision%29))
  (bind _output_get (Variables|/Game/Core/Data/SAV_Settings.SAV_Settings_C|SetSoundFXVolume (Variables|Settings|GetSettings) NewVolume))
  (Audio|SetSoundMixClassOverride "/Game/Audio/MIX_Main.MIX_Main" "/Game/Audio/SC_Sound.SC_Sound" _output_get 1.0 0.1 true)
  (Audio|PushSoundMixModifier "/Game/Audio/MIX_Main.MIX_Main")
  (Settings|SaveSettings))

(fn SetInitialVolumes
  (Class|GameplayStatics|SetBaseSoundMix "/Game/Audio/MIX_Main.MIX_Main")
  (ApplySettings|UpdateSoundVolume (Variables|/Game/Core/Data/SAV_Settings.SAV_Settings_C|GetSoundFXVolume (Variables|Settings|GetSettings)))
  (ApplySettings|UpdateMusicVolume (Variables|/Game/Core/Data/SAV_Settings.SAV_Settings_C|GetMusicVolume (Variables|Settings|GetSettings))))