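; Lobby platform actor representing one player slot, with a character and a widget button for opening the friend list.
; On the server it links the button to itself and finds the shared BP_FriendList, which it moves to its own location when shown.
; SpawnCharacter stores the controller, has GM_Lobby select the default class and hides the button and local list.
; Clear destroys the character and restores the button.
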(event Custom|SpawnCharacter
  (params (PC :type Player%20Controller%20Object%20Reference))
  (bind _friendlistref (Variables|Default|GetFriendlistRef))
  (bind _friendlistref_2 (Variables|Default|GetFriendlistRef))
  (bind _output_get (Variables|Default|SetPC PC))
  (Default|SelectCharacterClassbyIndex (.AsGM%20Lobby (Utilities|Casting|CastToGM_Lobby (Game|GetGameMode))) _output_get)
  (Rendering|SetVisibility (Variables|Default|GetOpenFriendlistButton) false false)
  (Utilities|IsValid _friendlistref_2
    (:Is%20Valid
      (if (Utilities|Operators|EqualEqual (Transformation|GetWorldLocation (Variables|Default|GetFriendListLocation)) (Transformation|GetActorLocation _friendlistref_2) 1.0)
        (Utilities|IsValid _friendlistref
          (:Is%20Valid
            (Default|Show _friendlistref false)))))))

(event Custom|Clear
  (Variables|Default|SetPC 0)
  (Utilities|IsValid (Variables|Default|GetCurrentCharacter)
    (:Is%20Valid
      (Actor|DestroyActor (Variables|Default|GetCurrentCharacter))
      (Variables|Default|SetCurrentCharacter 0))
    (:Is%20Not%20Valid
      _))
  (Rendering|SetVisibility (Variables|Default|GetOpenFriendlistButton) true false))

(event EventBeginPlay
  (CallFunction|SetupServer))

(fn ConstructionScript)

(fn ShowFriendlist
  (params (bShow :type Boolean))
  (bind _openfriendlistbutton (Variables|Default|GetOpenFriendlistButton))
  (bind _friendlistref (Variables|Default|GetFriendlistRef))
  (bind _friendlistref_2 (Variables|Default|GetFriendlistRef))
  (bind _returnvalue (UserInterface|GetWidget _openfriendlistbutton))
  (if bShow
    (Widget|SetVisibility _returnvalue "Collapsed")
    (Utilities|IsValid _friendlistref_2
      (:Is%20Valid
        (Transformation|SetActorLocation _friendlistref_2 (Transformation|GetWorldLocation (Variables|Default|GetFriendListLocation)) false false)
        (Utilities|IsValid _friendlistref
          (:Is%20Valid
            (Default|Show _friendlistref true self)))))
    (else
      (Widget|SetVisibility _returnvalue "Visible"))))

(fn SetupServer
  (if (Networking|IsServer)
    (bind _returnvalue (Actor|GetActorOfClass "/Game/Core/Lobby/BP_FriendList.BP_FriendList_C"))
    (Variables|Default|SetFriendlistRef _returnvalue)
    (bind _aswbp_open_friendlist_button (Utilities|Casting|CastToWBP_OpenFriendlistButton (UserInterface|GetWidget (Variables|Default|GetOpenFriendlistButton))))
    (Variables|/Game/UI/Widgets/Lobby/WBP_OpenFriendlistButton.WBP_OpenFriendlistButton_C|SetLobbyPlayerPlatformRef _aswbp_open_friendlist_button self)
    (Rendering|SetVisibility (Variables|Default|GetOpenFriendlistButton) true false)))