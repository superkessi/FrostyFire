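; Lobby friend list actor that is shown on behalf of a lobby player platform and hides itself when the mouse moves away.
; Show toggles visibility and tracks the requesting platform, turning off the friend list on the previously stored one.
; Each tick while visible, it projects the mouse ray out to the actor's distance and hides if that point falls outside FallOffRadius of the actor.
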(event EventBeginPlay)

(event Collision|EventActorBeginOverlap
  (params (OtherActor :type Actor%20Object%20Reference)))

(event EventTick
  (params (DeltaSeconds :type Float%20%28single-precision%29))
  (CallFunction|ChecktoHideFriendlist))

(fn ConstructionScript)

(fn Show
  (params (bShow :type Boolean) (FromLobbyPlayerPlatform :type BP%20Lobby%20Player%20Platform%20Object%20Reference))
  (if bShow
    (Rendering|SetActorHiddenInGame false)
    (Utilities|IsValid (Variables|Default|GetLastLobbyPlayerPlatform)
      (:Is%20Valid
        (Default|ShowFriendlist (Variables|Default|GetLastLobbyPlayerPlatform) false))
      (:Is%20Not%20Valid
        _))
    (Variables|Default|SetLastLobbyPlayerPlatform FromLobbyPlayerPlatform)
    (else
      (Rendering|SetActorHiddenInGame true)
      (Utilities|IsValid (Variables|Default|GetLastLobbyPlayerPlatform)
        (:Is%20Valid
          (Default|ShowFriendlist (Variables|Default|GetLastLobbyPlayerPlatform) false))
        (:Is%20Not%20Valid
          _))
      (Variables|Default|SetLastLobbyPlayerPlatform 0))))

(fn ChecktoHideFriendlist
  (bind _returnvalue (Game|GetPlayerController 0))
  (bind (_worldlocation _worlddirection) (Game|Player|ConvertMouseLocationToWorldSpace _returnvalue))
  (if (not (Variables|Rendering|GetbHidden))
    (if (not (Utilities|Operators|EqualEqual (+ _worldlocation (* _worlddirection (Math|Vector|Distance(Vector) (Transformation|GetActorLocation) _worldlocation))) (Transformation|GetActorLocation) (Variables|Default|GetFallOffRadius)))
      (CallFunction|Show false))))