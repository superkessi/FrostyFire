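; Player controller that handles local input setup, death and respawn flow, and UI focus for the player.
; On death the client deactivates character movement and focuses the game-over widget, while a guarded one-second server timer asks GM_Base to respawn the player.
; Pause, scoreboard, hit feedback and hitmarker are relayed through event dispatchers, with hits also shaking the camera.
; Focus helpers switch input mode, cursor and character movement together.
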(event Custom|Client_OnPlayerDied
  ;[0.009199 0.07242 0.4678] RPC's
  (Components|Activation|Deactivate (Variables|/Script/Engine.Character|GetCharacterMovement (Getter|GetCharacter)))
  ;;[0.8281 0 0.07523] REF!!!!!!!
  (Widget|FocusWidget (Variables|/Game/UI/Widgets/Ingame/WBP_Menus_Base.WBP_Menus_Base_C|GetGameOverScoreWidget (Variables|/Game/UI/HUD_Base.HUD_Base_C|GetMenuWidgetRef (Getter|GetHUDBase)))))

(event Custom|Server_StartRespawnTimer
  (if (not (Variables|Default|GetIsRespawning))
    (Variables|Default|SetIsRespawning true)
    (Utilities|Time|SetTimerbyEvent (delegate Custom|Server_RespawnTimerFinished) 1.0)))

(event Custom|Server_RespawnTimerFinished
  (Variables|Default|SetIsRespawning false)
  (bind _asgm_base (Utilities|Casting|CastToGM_Base (Game|GetGameMode)))
  (Default|RespawnPlayer _asgm_base (.AsBP%20Player%20State (Utilities|Casting|CastToBP_PlayerState (Variables|Default|GetPlayerState)))))

(event Input|EnhancedActionEvents|EnhancedInputActionIA_ToggleGameMenu
  (params (ActionValue :type Boolean) (ElapsedSeconds :type Float%20%28double-precision%29) (TriggeredSeconds :type Float%20%28double-precision%29) (InputAction :type Input%20Action%20Object%20Reference :default "/Game/Core/Input/Actions/IA_ToggleGameMenu.IA_ToggleGameMenu"))
  ;[0.4844 0.3843 0] Toggle Pause Menu
  (:Started
    (Widget|TogglePauseMenu)))

(event Input|EnhancedActionEvents|EnhancedInputActionIA_ShowScoreboard
  (params (ActionValue :type Boolean) (ElapsedSeconds :type Float%20%28double-precision%29) (TriggeredSeconds :type Float%20%28double-precision%29) (InputAction :type Input%20Action%20Object%20Reference :default "/Game/Core/Input/Actions/IA_ShowScoreboard.IA_ShowScoreboard"))
  ;[0.4844 0.3843 0] ScoreBoard
  (:Started
    (Default|CallOnToggleScoreboard :!label _label))
  (:Canceled
    (goto _label))
  (:Completed
    (goto _label)))

(event EventBeginPlay
  ;[0.02761 0.07292 0.01699] SetUp
  (if (Pawn|IsLocalController)
    (Setup|SetupInputSystem)))

(fn ConstructionScript)

(fn FocusWidget
  (params (WIdget :type Widget%20Object%20Reference))
  (bind _character (Getter|GetCharacter))
  (Input|SetInputModeUIOnly self WIdget "DoNotLock" false)
  (Variables|Default|SetbShowMouseCursor true)
  (Utilities|IsValid _character
    (:Is%20Valid
      (Variables|/Script/FrostyFire.FrostyFireCharacter|SetbCanMove _character false))))

(fn FocusGame
  (bind _character (Getter|GetCharacter))
  (Input|SetInputModeGameOnly self false)
  (Variables|Default|SetbShowMouseCursor false)
  (Class|WidgetBlueprintLibrary|SetFocustoGameViewport)
  (Utilities|IsValid _character
    (:Is%20Valid
      (Variables|/Script/FrostyFire.FrostyFireCharacter|SetbCanMove _character true))))

(fn TogglePauseMenu
  (Default|CallOnTogglePauseMenu))

(fn SetupIngameUI)

(fn PlayLocalHitIndicator
  (Default|CallOnPlayHitFeedback)
  (Hit|PlayHitCameraShake))

(fn PlayHitCameraShake
  (CameraShakes|StartCameraShake (Game|GetPlayerCameraManager 0) "/Game/Testing/Resi/BP_CameraShakeTest.BP_CameraShakeTest_C" 1.0 "CameraLocal" "0, 0, 0"))

(fn GetHUDBase
  (return (.AsHUD%20Base (Utilities|Casting|CastToHUD_Base (HUD|GetHUD)))))

(fn ShowCursor
  (params (Show :type Boolean))
  (bind _self self)
  (Input|SetInputModeGameOnly _self false)
  (Variables|Default|SetbShowMouseCursor _self Show))

(fn ResetPlayerController
  (Widget|FocusGame))

(fn SetupInputSystem
  (bind _self self)
  (bind _returnvalue (PlayerController|LocalPlayerSubsystems|GetEnhancedInputLocalPlayerSubsystem _self))
  (bind _returnvalue_2 (Class|EnhancedInputSubsystemInterface|GetUserSettings _returnvalue))
  (Utilities|IsValid _returnvalue
    (:Is%20Valid
      (Input|AddMappingContext _returnvalue "/Game/Core/Input/IMC_Default.IMC_Default" 0 "(bIgnoreAllPressedKeysUntilRelease=True,bForceImmediately=False,bNotifyUserSettings=False)")
      (if (not (Class|EnhancedInputUserSettings|IsMappingContextRegistered _returnvalue_2 "/Game/Core/Input/IMC_Default.IMC_Default"))
        (Class|EnhancedInputUserSettings|RegisterInputMappingContext _returnvalue_2 "/Game/Core/Input/IMC_Default.IMC_Default")))))

(fn GetGameStateBase
  (bind _asgs_base (Utilities|Casting|CastToGS_Base (Game|GetGameState)))
  (return _asgs_base))

(fn GetCharacter
  (bind _asbp_player_character (Utilities|Casting|CastToBP_PlayerCharacter (Pawn|GetControlledPawn)))
  (return _asbp_player_character))

(fn GetCurrentMatchPhase
  (return (Variables|/Game/Core/Game/GS_Base.GS_Base_C|GetMatchPhase (.AsGS%20Base (Utilities|Casting|CastToGS_Base (Game|GetGameState))))))

(fn PlayHitmarker
  (params (PlayerKilled? :type Boolean))
  (Default|CallOnPlayHitmaker PlayerKilled?))