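; Player State Blueprint that tracks a player's lives, kill score, deaths and dead flag.
; Helper functions add score, subtract damage from lives, mark the player dead and count a death at zero lives, and reset either all stats or only lives and the dead flag.
; Each stat uses a RepNotify that, like BeginPlay, calls OnStatsChanges to broadcast updates.
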(event EventBeginPlay
  (Default|CallOnStatsChanges))

(fn ConstructionScript)

(fn OnRepLives
  (Default|CallOnStatsChanges))

(fn OnRepKillScore
  (Default|CallOnStatsChanges))

(fn AddScore
  (params (Points :type Integer))
  (Variables|Default|SetKillScore (+ Points (Variables|Default|GetKillScore))))

(fn OnRepDeaths
  (Default|CallOnStatsChanges))

(fn AddDeath
  (Variables|Default|SetDeaths (+ (Variables|Default|GetDeaths) 1)))

(fn SubstactLive
  (params (Damage :type Integer))
  (Variables|Default|SetLives (- (Variables|Default|GetLives) Damage))
  ;[0.15 0.15 0.15 0.5] Dings
  (if (<= (Variables|Default|GetLives) 0)
    (Variables|Default|SetIsDead true)
    (Hit|AddDeath)))

(fn OnRepIsDead
  (Default|CallOnStatsChanges))

(fn ResetPlayerStats
  (Variables|Default|SetIsDead false)
  (Variables|Default|SetLives 3)
  (Variables|Default|SetKillScore 0)
  (Variables|Default|SetDeaths 0))

(fn ResetPlayerLives
  (Variables|Default|SetIsDead false)
  (Variables|Default|SetLives 3))