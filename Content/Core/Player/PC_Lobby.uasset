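; Lobby player controller that creates the local player's lobby UI and relays name, ready status and character choice to GM_Lobby.
; Ready toggles and name events push player info through UpdatePlayerLobbyInfo, with a delayed retry event available.
; Character selection cycles through eight class indices with a looping MultiGate that starts at the second entry.
; Match start shows the UI's loading screen and disables input.
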(event Custom|TryAgainUpdatingLobbyInfo
  (Utilities|FlowControl|Delay 0.1)
  (bind _asgm_lobby (Utilities|Casting|CastToGM_Lobby (Game|GetGameMode)))
  (Default|UpdatePlayerLobbyInfo _asgm_lobby self))

(event Custom|SetPlayerNameOnServer
  (params (PlayerName :type Text))
  (bind _asgm_lobby (Utilities|Casting|CastToGM_Lobby (Game|GetGameMode)))
  (Default|UpdatePlayerLobbyInfo _asgm_lobby self))

(event Custom|ToggleReadyStatusOnServer
  (bind _playerlobbyinfopc (Variables|Default|GetPlayerLobbyInfoPC))
  (Utilities|Struct|SetmembersinF_PlayerLobbyInfo _playerlobbyinfopc (not (.bReady (Utilities|Struct|BreakF_PlayerLobbyInfo _playerlobbyinfopc))))
  (bind _asgm_lobby (Utilities|Casting|CastToGM_Lobby (Game|GetGameMode)))
  (Default|UpdatePlayerLobbyInfo _asgm_lobby self))

(event Custom|OnStartMatch
  (Default|ShowLoadingScreen (Variables|Default|GetLobbyUI_ref))
  (Input|DisableInput self))

(event Custom|SelectCharOnServer
  (Utilities|FlowControl|MultiGate false true 1
    (:Out%200
      (Default|SelectCharacterClassbyIndex (Variables|Default|GetLobbyGM_ref) self))
    (:Out%201
      (Default|SelectCharacterClassbyIndex (Variables|Default|GetLobbyGM_ref) self 1))
    (:Out%202
      (Default|SelectCharacterClassbyIndex (Variables|Default|GetLobbyGM_ref) self 2))
    (:Out%203
      (Default|SelectCharacterClassbyIndex (Variables|Default|GetLobbyGM_ref) self 3))
    (:Out%204
      (Default|SelectCharacterClassbyIndex (Variables|Default|GetLobbyGM_ref) self 4))
    (:Out%205
      (Default|SelectCharacterClassbyIndex (Variables|Default|GetLobbyGM_ref) self 5))
    (:Out%206
      (Default|SelectCharacterClassbyIndex (Variables|Default|GetLobbyGM_ref) self 6))
    (:Out%207
      (Default|SelectCharacterClassbyIndex (Variables|Default|GetLobbyGM_ref) self 7))))

(event EventBeginPlay
  (CallFunction|SetUp)
  (Variables|Default|SetLobbyGM_ref (.AsGM%20Lobby (Utilities|Casting|CastToGM_Lobby (Game|GetGameMode)))))

(event EventPossess
  (params (PossessedPawn :type Pawn%20Object%20Reference)))

(fn ConstructionScript)

(fn SetUp
  (if (Pawn|IsLocalPlayerController)
    (Variables|Default|SetbShowMouseCursor true)
    (Input|SetInputModeGameandUI self 0 "DoNotLock" false false)
    (bind _returnvalue (UserInterface|CreateWidget "/Game/UI/Widgets/Lobby/WBP_LobbyUI.WBP_LobbyUI_C"))
    (bind _output_get (Variables|Default|SetLobbyUI_ref _returnvalue))
    (UserInterface|Viewport|AddtoViewport _output_get 0)
    (CallFunction|SetPlayerNameonServer)))