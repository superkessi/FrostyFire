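; Player character for a multiplayer snowball fight, with hold-to-charge throws, timed reloads, hit reactions and ragdoll death.
; Game state match phases toggle movement and input, while tuning values come from PlayerStatsData.
; Throws aim along the camera and spawn BP_Snowball via server RPC; montages for both meshes relay through server-to-multicast events.
; Hits go to the game mode on authority, and replicated FaceChange swaps facial expressions through material UV offsets.
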(event Custom|Client_Reload
  ;[0.009199 0.07242 0.4678] Reload
  (Variables|Locals|SetCurrentAmmo (Variables|Values|GetMaxAmmo)))

(event Custom|Client_UpdateAmmo
  ;[0.02502 0.15 0.03519 0.5] Throw
  ;;[0.15 0.15 0.15 0.5] Spawn Snowball RPC
  (Variables|Locals|SetCurrentAmmo (- (Variables|Locals|GetCurrentAmmo) 1)))

(event Custom|MC_PlayThrowMontage
  ;[0.02502 0.15 0.03519 0.5] Throw
  ;;[0.15 0.15 0.15 0.5] Throw Anim RPCs
  (Animation|Montage|PlayMontage (Variables|Character|GetMesh) "/Game/Testing/Hannah/AM_Player_Wurf.AM_Player_Wurf" 1.0 0.0 "LoopAim"
    (:then
      (Animation|Montage|PlayMontage (Variables|Default|GetFirstPersonMesh) "/Game/Testing/Hannah/AM_Player_Wurf.AM_Player_Wurf" 1.0 0.0 "LoopAim"))))

(event Custom|Server_PlayThrowEnd
  ;[0.02502 0.15 0.03519 0.5] Throw
  ;;[0.15 0.15 0.15 0.5] Throw Anim RPCs
  (CallFunction|MCPlayThrowEnd))

(event Custom|MC_PlayThrowEnd
  ;[0.02502 0.15 0.03519 0.5] Throw
  ;;[0.15 0.15 0.15 0.5] Throw Anim RPCs
  (Animation|Montage|PlayMontage (Variables|Character|GetMesh) "/Game/Testing/Hannah/AM_Player_Wurf.AM_Player_Wurf" 1.0 0.0 "Throw"
    (:then
      (Animation|Montage|PlayMontage (Variables|Default|GetFirstPersonMesh) "/Game/Testing/Hannah/AM_Player_Wurf.AM_Player_Wurf" 1.0 0.0 "Throw"))))

(event Custom|Client_PlayHitIndicator
  (bind _player_controller (Getter|GetPlayerController))
  ;[0.8281 0 0.07523] Hit Reactions
  (Utilities|IsValid _player_controller
    (:Is%20Valid
      (Default|PlayLocalHitIndicator _player_controller))))

(event Custom|PlayRagdoll
  ;[0.15 0.15 0.15 0.5] Ragdoll RPCs
  (Collision|SetCollisionProfileName (Variables|Character|GetMesh) "Ragdoll" true :!class /Script/Engine.PrimitiveComponent)
  (Class|SkeletalMeshComponent|SetPhysicsBlendWeight (Variables|Character|GetMesh) 1.0))

(event Custom|PlayHitMarker
  (params (PlayerKilled? :type Boolean))
  (Default|PlayHitmarker (Getter|GetPlayerController) PlayerKilled?))

(event Custom|MC_PlayDeathFeedback
  ;[0 0 0 0.5] Death
  (CallFunction|ClientPlayHitIndicator)
  (Variables|Default|SetIsAlive false)
  (Class|FrostyFireCharacter|SetCanMove false)
  (CallFunction|PlayHitParticles)
  (CallFunction|PlayRagdoll)
  (Collision|SetCollisionEnabled (Variables|Default|GetCapsuleComponent) "NoCollision")
  (CallFunction|MCFacechange 5))

(event Custom|Server_SetBallPreview_TP
  (params (StaticMesh :type Static%20Mesh%20Component%20Object%20Reference) (SetHidden :type Boolean))
  ;[0.02502 0.15 0.03519 0.5] Throw
  ;;[0.15 0.15 0.15 0.5] Snowball Preview RPCs
  (CallFunction|MCSetBallPreview StaticMesh SetHidden))

(event Custom|MC_Facechange
  (params (FaceChange :type Integer))
  ;[0.8281 0 0.07523] Hit Reactions
  (Variables|Default|SetFaceChange FaceChange))

(event Custom|MC_SetBallPreview
  (params (SnowballMesh :type Static%20Mesh%20Component%20Object%20Reference) (SetHidden :type Boolean))
  ;[0.02502 0.15 0.03519 0.5] Throw
  ;;[0.15 0.15 0.15 0.5] Snowball Preview RPCs
  (Development|SetHiddeninGame SnowballMesh SetHidden false))

(event Custom|Server_SpawnSnowball
  (params (SpawnTransform :type Transform) (ThrowSpeed :type Float%20%28double-precision%29) (ThrowVelo :type Vector))
  ;[0.02502 0.15 0.03519 0.5] Throw
  ;;[0.15 0.15 0.15 0.5] Spawn Snowball RPC
  (Throw|SpawnSnoball SpawnTransform ThrowSpeed ThrowVelo))

(event Custom|PlayHitParticles
  ;[0.8281 0 0.07523] Hit Reactions
  (Components|Activation|Activate (Variables|Default|GetHitParticles) false))

(event Custom|PlayHitAnim
  ;[0.8281 0 0.07523] Hit Reactions
  (Animation|PlayAnimMontage "/Game/Animations/AS_AM_Animations/AM_Hit_Reaction.AM_Hit_Reaction" 1.0 "None"))

(event Custom|MC_PlayReloadEnd
  ;[0.02502 0.15 0.03519 0.5] Throw
  ;;[0.15 0.15 0.15 0.5] Reload Anim RPCs
  (Animation|Montage|PlayMontage (Variables|Character|GetMesh) "/Game/Testing/Hannah/AM_Player_Reload.AM_Player_Reload" 1.0 0.0 "End"
    (:then
      (Animation|Montage|PlayMontage (Variables|Default|GetFirstPersonMesh) "/Game/Testing/Hannah/AM_Player_Reload.AM_Player_Reload" 1.0 0.0 "End"))))

(event Custom|MC_PlayHitFeedback
  ;[0.1302 0.02231 0] Hit
  (CallFunction|ClientPlayHitIndicator)
  (CallFunction|PlayHitParticles)
  (CallFunction|PlayHitAnim)
  (CallFunction|MCFacechange 6)
  (Utilities|FlowControl|Delay 1.0)
  (CallFunction|MCFacechange 1))

(event Custom|Server_PlayReloadEnd
  ;[0.02502 0.15 0.03519 0.5] Throw
  ;;[0.15 0.15 0.15 0.5] Reload Anim RPCs
  (CallFunction|MCPlayReloadEnd))

(event Custom|Server_PlayReloadMontage
  ;[0.02502 0.15 0.03519 0.5] Throw
  ;;[0.15 0.15 0.15 0.5] Reload Anim RPCs
  (CallFunction|MCPlayReloadMontrage))

(event Custom|MC_PlayReloadMontrage
  ;[0.02502 0.15 0.03519 0.5] Throw
  ;;[0.15 0.15 0.15 0.5] Reload Anim RPCs
  (Animation|Montage|PlayMontage (Variables|Character|GetMesh) "/Game/Testing/Hannah/AM_Player_Reload.AM_Player_Reload" 1.0 0.0 "Reload:Loop"
    (:then
      (Animation|Montage|PlayMontage (Variables|Default|GetFirstPersonMesh) "/Game/Testing/Hannah/AM_Player_Reload.AM_Player_Reload" 1.0 0.0 "Reload:Loop"))))

(event Custom|ReactToMatchPhase
  (params (Phase :type ENUM_MatchPhases%20Enum :default "NewEnumerator0"))
  ;[0.1302 0.02231 0] Game States
  (switch Utilities|FlowControl|Switch|SwitchonENUM_MatchPhases Phase
    (:NewEnumerator0
      (GameStates|ReacttoWaiting))
    (:NewEnumerator1
      (GameStates|ReacttoCountdown))
    (:NewEnumerator2
      (GameStates|ReacttoPlaying))
    (:NewEnumerator3
      (GameStates|ReacttoGameOver))))

(event Custom|Server_PlayThrowMontage
  ;[0.02502 0.15 0.03519 0.5] Throw
  ;;[0.15 0.15 0.15 0.5] Throw Anim RPCs
  (CallFunction|MCPlayThrowMontage))

(event Input|EnhancedActionEvents|EnhancedInputActionIA_Reload
  (params (ActionValue :type Boolean) (ElapsedSeconds :type Float%20%28double-precision%29) (TriggeredSeconds :type Float%20%28double-precision%29) (InputAction :type Input%20Action%20Object%20Reference :default "/Game/Core/Input/Actions/IA_Reload.IA_Reload"))
  ;[0.009199 0.07242 0.4678] Reload
  (if (not (Variables|Locals|GetIsReloading))
    ;;[0.4844 0.3843 0] REF
    (if (not (> (Variables|Locals|GetCurrentAmmo) 0))
      (Reload|HandleReloadInputStarted)
      (bind _progress (Timeline|ReloadTimeLine PlayFromStart)
        (:Update
          (Reload|UpdateReloadCharge _progress))
        (:Finished
          (Reload|HandleReloadFinished))))))

(event Input|EnhancedActionEvents|EnhancedInputActionIA_Throw
  (params (ActionValue :type Boolean) (ElapsedSeconds :type Float%20%28double-precision%29) (TriggeredSeconds :type Float%20%28double-precision%29) (InputAction :type Input%20Action%20Object%20Reference :default "/Game/Core/Input/Actions/IA_Throw.IA_Throw"))
  ;[0.02502 0.15 0.03519 0.5] Throw
  (:Started
    (Throw|HandleThrowInputStarted))
  (:Ongoing
    (Throw|HandleThrowInputOngoing ElapsedSeconds))
  (:Completed
    (Throw|HandleThrowInputCompleted ElapsedSeconds)))

(event EventOnPlayerStateReady
  ;[0.772 0.8646 0] SetUp
  (Setter|SetupInitialMouseSens))

(event EventPossessed
  (params (NewController :type Controller%20Object%20Reference))
  (bind _asgs_base (Getter|GetGameState))
  ;[0.772 0.8646 0] SetUp
  (EventDispatchers|BindEventtoOnMatchPhaseChanged _asgs_base (delegate Custom|ReactToMatchPhase))
  (CallFunction|ReacttoMatchPhase (Variables|/Game/Core/Game/GS_Base.GS_Base_C|GetMatchPhase _asgs_base))
  (Rendering|SetVisibility (Variables|Default|GetIngameNameTag) true false))

(event EventOnSnowballHit
  (params (Attacker%20Controller :type BP%20Player%20Controller%20Object%20Reference))
  ;[0.1302 0.02231 0] Hit
  (Networking|SwitchHasAuthority
    (:Authority
      (Default|HandlePlayerHit (Getter|GetGameModeBase) Attacker%20Controller (Getter|GetPlayerController)))))

(event EventUnpossessed
  (params (OldController :type Controller%20Object%20Reference))
  ;[0.772 0.8646 0] Clean Up
  (EventDispatchers|UnbindEventfromOnMatchPhaseChanged (Getter|GetGameState) (delegate Custom|ReactToMatchPhase))
  (Rendering|SetVisibility (Variables|Default|GetIngameNameTag) false false)
  (Utilities|FlowControl|Delay 3.0)
  (Actor|DestroyActor))

(event EventTick
  (params (DeltaSeconds :type Float%20%28single-precision%29))
  ;[0.8281 0 0.07523] Tick
  (Updates|UpdateFloatingTextRotation))

(event EventBeginPlay
  ;[0.8281 0 0.07523] Begin Play
  (Setter|SetupIngameNameTag)
  (Setter|SetMouseSens)
  (Variables|Default|SetIsAlive true))

(fn ConstructionScript
  (bind _returnvalue (Rendering|Material|CreateDynamicMaterialInstance (Variables|Default|GetFace) 0 (Rendering|Material|GetMaterial (Variables|Default|GetFace) 0) "None" :!class /Script/Engine.PrimitiveComponent))
  (bind _output_get (Variables|Default|SetFaceExpression _returnvalue))
  (Rendering|Material|SetMaterial (Variables|Default|GetFace) 0 _output_get)
  (Setter|SetPlayerData))

(fn CanShoot
  (if (> (Variables|Locals|GetCurrentAmmo) 0)
    (bind _asbp_player_state (Utilities|Casting|CastToBP_PlayerState (Variables|Default|GetPlayerState)))
    (if (Variables|/Game/Core/Player/BP_PlayerState.BP_PlayerState_C|GetIsDead _asbp_player_state)
      _
      (elif (Variables|Default|GetIsAlive)
        (return true)
        (else
          _))))
  (return false))

(fn UpdateCharge
  (params (Value :type Float%20%28double-precision%29))
  (Variables|/Game/Core/Player/BP_PlayerController.BP_PlayerController_C|SetThrowChargeValue (Getter|GetPlayerController) (/ (Math|Float|Clamp(Float) Value 0.0 (Variables|Values|GetMaxChargeTime)) (Variables|Values|GetMaxChargeTime))))

(fn UpdateReloadCharge
  (params (Percentage :type Float%20%28single-precision%29))
  (Variables|/Game/Core/Player/BP_PlayerController.BP_PlayerController_C|SetReloadChrageValue (Getter|GetPlayerController) Percentage))

(fn GetMaxHealth
  (return (Variables|/Game/Core/Player/DA_PlayerStats.DA_PlayerStats_C|GetMaxHealth (Variables|Default|GetPlayerStatsData))))

(fn GetCurrentMatchPhase
  (bind _asgs_base (Utilities|Casting|CastToGS_Base (Game|GetGameState)))
  (return (Variables|/Game/Core/Game/GS_Base.GS_Base_C|GetMatchPhase _asgs_base)))

(fn SetBallPreviewVisibility
  (params (SetHidden :type Boolean))
  (CallFunction|ServerSetBallPreviewTP (Variables|Default|GetSnowballPreview_TP) SetHidden)
  (Development|SetHiddeninGame (Variables|Default|GetSnowballPreview_FP) SetHidden false))

(fn Die)

(fn GetPlayerController
  (bind _asbp_player_controller (Utilities|Casting|CastToBP_PlayerController (Pawn|GetController)))
  (return _asbp_player_controller))

(fn ReacttoWaiting
  (CallFunction|ActivatePlayer false)
  (Default|ShowCursor (Getter|GetPlayerController) true))

(fn ReacttoCountdown
  (CallFunction|ActivatePlayer false)
  (Default|FocusGame (Getter|GetPlayerController))
  (Default|ShowCursor (Getter|GetPlayerController) false))

(fn ReacttoPlaying
  (CallFunction|ActivatePlayer true))

(fn ReacttoGameOver
  (CallFunction|ActivatePlayer false)
  (Default|CallOnGameOver))

(fn HandleThrowInputCompleted
  (params (InputPin :type Float%20%28double-precision%29))
  (bind _throwspeed (Variables|Locals|GetThrowSpeed))
  (if (Throw|CanShoot)
    (if (Variables|Default|GetIsCharging)
      (Throw|UpdateCharge 0.0)
      (Utilities|SetAimpoint
        (:Continue
          (CallFunction|ServerPlayThrowEnd)
          (Throw|SetBallPreviewVisibility true)
          (Utilities|CalculateThrowSpeed InputPin
            (:%20%20
              (bind _spawntransform (Utilities|GetSnowballSpawnPoint)
                (:%20%20
                  (CallFunction|ServerSpawnSnowball _spawntransform _throwspeed (* _throwspeed (Variables|Locals|GetAimDirection)))
                  (CallFunction|ClientUpdateAmmo)
                  (Variables|Default|SetIsCharging false))))))))))

(fn HandleThrowInputStarted
  (if (Throw|CanShoot)
    (CallFunction|ServerPlayThrowMontage)
    (Variables|Default|SetIsCharging true)))

(fn HandleThrowInputOngoing
  (params (InputPin :type Float%20%28double-precision%29))
  (if (Variables|Default|GetIsCharging)
    (if (Throw|CanShoot)
      (Throw|UpdateCharge InputPin)
      (else
        (Throw|UpdateCharge 0.0)
        (Variables|Default|SetIsCharging false)))))

(fn SpawnSnoball
  (params (SpawnTransform :type Transform) (ThrowSpeed :type Float%20%28double-precision%29) (ThrowVelo :type Vector))
  (bind _self self)
  (bind _returnvalue (Game|SpawnActorfromClass "/Game/Gameplay/Actors/BP_Snowball.BP_Snowball_C" SpawnTransform "Undefined" "MultiplyWithRoot" _self _self))
  (Variables|/Script/Engine.ProjectileMovementComponent|SetInitialSpeed (Variables|/Script/FrostyFire.Snowball|GetProjectileMovementComponent _returnvalue) ThrowSpeed)
  (Game|Components|ProjectileMovement|SetVelocityinLocalSpace (Variables|/Script/FrostyFire.Snowball|GetProjectileMovementComponent _returnvalue) ThrowVelo))

(fn HandleReloadInputStarted
  (Variables|Locals|SetIsReloading true)
  (Components|Timeline|SetPlayRate (Variables|Default|GetReloadTimeLine) (/ 1.0 (Variables|Values|GetReloadTime)))
  (CallFunction|ServerPlayReloadMontage)
  (Throw|SetBallPreviewVisibility false))

(fn HandleReloadFinished
  (Reload|UpdateReloadCharge 0.0)
  (Variables|Locals|SetIsReloading false)
  (CallFunction|ClientReload)
  (CallFunction|ServerPlayReloadEnd))

(fn ActivatePlayer
  (params (Activate :type Boolean))
  (bind _player_controller (Getter|GetPlayerController))
  (if Activate
    (Class|FrostyFireCharacter|SetCanMove true)
    (Utilities|IsValid _player_controller
      (:Is%20Valid
        (Input|EnableInput _player_controller)
        (Default|FocusGame _player_controller)))
    (else
      (Class|FrostyFireCharacter|SetCanMove false)
      (Input|DisableInput (Getter|GetPlayerController)))))

(fn OnRepPlayerLobbyInfo
  (bind _lobbynametag (Variables|Default|GetLobbyNameTag))
  (bind _returnvalue (UserInterface|GetWidget _lobbynametag))
  (Utilities|IsValid _returnvalue
    (:Is%20Valid
      (bind _aswbp_player_lobby_info (Utilities|Casting|CastToWBP_PlayerLobbyInfo _returnvalue))
      (Default|Update _aswbp_player_lobby_info (Variables|Default|GetPlayerLobbyInfo))
      (Rendering|SetVisibility (Variables|Default|GetLobbyNameTag) true false))
    (:Is%20Not%20Valid
      (Utilities|Time|SetTimerbyFunctionName 0 "OnRep_PlayerLobbyInfo" 0.1))))

(fn GetGameState
  (bind _asgs_base (Utilities|Casting|CastToGS_Base (Game|GetGameState))
    (:then
      _)
    (:CastFailed
      _))
  (return _asgs_base))

(fn OnRepFaceChange
  (Rendering|Material|SetVectorParameterValue (Variables|Default|GetFaceExpression) "UV Controls" (Utilities|Select :Index (Variables|Default|GetFaceChange) :Option%200 "" :Option%201 "(R=1.000000,G=1.000000,B=0.000000,A=0.000000)" :Option%202 "(R=1.000000,G=1.000000,B=0.502887,A=0.000000)" :Option%203 "(R=1.000000,G=1.000000,B=0.000000,A=0.333333)" :Option%204 "(R=1.000000,G=1.000000,B=0.502887,A=0.333333)" :Option%205 "(R=1.000000,G=1.000000,B=0.502887,A=0.666667)" :Option%206 "(R=1.000000,G=1.000000,B=0.000000,A=0.666667)") :!class /Script/Engine.MaterialInstanceDynamic))

(fn GetGameModeBase
  (bind _asgm_base (Utilities|Casting|CastToGM_Base (Game|GetGameMode))
    (:then
      _)
    (:CastFailed
      _))
  (return _asgm_base))

(fn UpdatePlayerLobbyInfo
  (params (PlayerLobbyInfo :type F%20Player%20Lobby%20Info%20Structure))
  (Variables|Default|SetPlayerLobbyInfo PlayerLobbyInfo))

(fn UpdateFloatingTextRotation
  (Transformation|SetWorldRotation (Variables|Default|GetIngameNameTag) (Math|Rotator|FindLookatRotation (Transformation|GetWorldLocation (Variables|Default|GetIngameNameTag)) (Camera|GetCameraLocation (Variables|/Script/Engine.PlayerController|GetPlayerCameraManager (Game|GetPlayerController 0)))) false false))

(fn SetupInitialMouseSens
  (bind _asbp_afgame_instance (Utilities|Casting|CastToBP_AFGameInstance (Game|GetGameInstance))
    (:then
      (Default|UpdateMouseSens _asbp_afgame_instance (Variables|/Game/Core/Data/SAV_Settings.SAV_Settings_C|GetMouseSensitivity (Variables|/Game/Core/Game/BP_AFGameInstance.BP_AFGameInstance_C|GetSettings _asbp_afgame_instance))))
    (:CastFailed
      (Development|PrintString "GameInstance cast failed"))))

(fn SetMouseSens
  (Variables|Default|SetMouseSensitivity (Variables|/Game/Core/Data/SAV_Settings.SAV_Settings_C|GetMouseSensitivity (Variables|/Game/Core/Game/BP_AFGameInstance.BP_AFGameInstance_C|GetSettings (.AsBP%20AFGame%20Instance (Utilities|Casting|CastToBP_AFGameInstance (Game|GetGameInstance)))))))

(fn SetPlayerData
  (bind _playerstatsdata (Variables|Default|GetPlayerStatsData))
  (Utilities|FlowControl|Sequence
    (:then_0
      (Variables|Values|SetMaxHealth (Variables|/Game/Core/Player/DA_PlayerStats.DA_PlayerStats_C|GetMaxHealth _playerstatsdata)))
    (:then_1
      (Variables|Values|SetMaxAmmo (Variables|/Game/Core/Player/DA_PlayerStats.DA_PlayerStats_C|GetMaxAmmo _playerstatsdata)))
    (:then_2
      (Variables|Values|SetMaxChargeTime (Variables|/Game/Core/Player/DA_PlayerStats.DA_PlayerStats_C|GetMaxChargeTime _playerstatsdata)))
    (:then_3
      (Variables|Values|SetMinThrowSpeed (Variables|/Game/Core/Player/DA_PlayerStats.DA_PlayerStats_C|GetMinThrowSpeed _playerstatsdata)))
    (:then_4
      (Variables|Values|SetMaxThrowSpeed (Variables|/Game/Core/Player/DA_PlayerStats.DA_PlayerStats_C|GetMaxThrowSpeed _playerstatsdata)))
    (:then_5
      (Variables|Values|SetMaxTraceDistance (Variables|/Game/Core/Player/DA_PlayerStats.DA_PlayerStats_C|GetMaxTraceDistance _playerstatsdata)))
    (:then_6
      (Variables|Values|SetReloadTime (Variables|/Game/Core/Player/DA_PlayerStats.DA_PlayerStats_C|GetReloadTime _playerstatsdata)))
    (:then_7
      (Variables|Values|SetSnowballSpawnOffset (Variables|/Game/Core/Player/DA_PlayerStats.DA_PlayerStats_C|GetSnowballSpawnOffset _playerstatsdata)))))

(fn SetupIngameNameTag
  (bind _aswbp_player_name_tag (Utilities|Casting|CastToWBP_PlayerNameTag (UserInterface|GetWidget (Variables|Default|GetIngameNameTag))))
  (Variables|/Game/UI/Widgets/Ingame/WBP_PlayerNameTag.WBP_PlayerNameTag_C|SetOwner _aswbp_player_name_tag self))